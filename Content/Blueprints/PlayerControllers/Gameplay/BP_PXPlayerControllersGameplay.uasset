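; Gameplay player controller that installs the default Enhanced Input mapping context and handles pausing.
; On BeginPlay it adds IMC_Default to the local player subsystem.
; The pause input action toggles a flag, creating and showing WBP_PXPauseMenu with Game and UI input, a visible cursor and paused game, or removing it and restoring game-only input.
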(event `self.ReceiveBeginPlay`
  (bind _returnvalue (subsystem `EnhancedInputLocalPlayerSubsystem`))
  (`/Engine/EditorBlueprintResources/StandardMacros.IsValid` _returnvalue
    (:`Is Valid`
      (`EnhancedInputSubsystemInterface.AddMappingContext` _returnvalue "/Game/Blueprints/Input/IMC_Default.IMC_Default" 0 (struct)))))

(event `EnhancedInput|/Game/Blueprints/Input/Actions/IA_PauseGame`
  (params (ActionValue :type Boolean) (ElapsedSeconds :type "Float (double-precision)") (TriggeredSeconds :type "Float (double-precision)") (InputAction :type "InputAction Object Reference" :default "/Game/Blueprints/Input/Actions/IA_PauseGame.IA_PauseGame"))
  (:`Started`
    (if (not (`self.IsPauseMenuOpened`))
      (set `self.IsPauseMenuOpened` true)
      (bind _returnvalue (`|CreateWidget` "/Game/Blueprints/UI/PauseMenu/WBP_PXPauseMenu.WBP_PXPauseMenu_C"))
      (bind _output_get (set `self.PauseMenuWidget` _returnvalue))
      (`UserWidget.AddToViewport` _output_get 0)
      (`WidgetBlueprintLibrary.SetInputMode_GameAndUIEx` self (`self.PauseMenuWidget`))
      (set `self.bShowMouseCursor` true)
      (`GameplayStatics.SetGamePaused` true)
      (else
        (set `self.IsPauseMenuOpened` false)
        (`Widget.RemoveFromParent` (`self.PauseMenuWidget`))
        (`WidgetBlueprintLibrary.SetInputMode_GameOnly` self)
        (set `self.bShowMouseCursor` false)
        (`GameplayStatics.SetGamePaused` false)))))

(fn `UserConstructionScript`)