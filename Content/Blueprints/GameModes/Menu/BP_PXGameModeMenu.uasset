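; Menu game mode that picks which screen to show when the menu level begins play.
; On the first visit it marks the game as started in the PX level subsystem and opens the main menu widget.
; On later visits it asks the score subsystem whether the high score was beaten, then opens either the celebration or end game widget.
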(event `self.ReceiveBeginPlay`
  (`parent.ReceiveBeginPlay`)
  (`self.OpenCorrectWidget`))

(fn `OpenCorrectWidget`
  (if (not (`PXLevelSubsystem.GetHasGameStarted` (subsystem `PXLevelSubsystem`)))
    ;[1 1 1] When open the game, open Main Menu
    (`PXLevelSubsystem.SetHasGameStarted` (subsystem `PXLevelSubsystem`) true)
    (bind _returnvalue (`|CreateWidget` "/Game/Blueprints/UI/Menu/MainMenu/WBP_PXMainMenuWidget.WBP_PXMainMenuWidget_C"))
    (`UserWidget.AddToViewport` _returnvalue 0)
    (elif (`PXScoreSubsystem.IsHighScoreBeaten` (subsystem `PXScoreSubsystem`))
      ;[1 1 1] When beat highscore, open Celebration
      (bind _returnvalue_2 (`|CreateWidget` "/Game/Blueprints/UI/Menu/Celebration/WBP_PXCelebrationWidget.WBP_PXCelebrationWidget_C"))
      (`UserWidget.AddToViewport` _returnvalue_2 0)
      (else
        ;[1 1 1] When do not beat highscore, open End Game
        (bind _returnvalue_3 (`|CreateWidget` "/Game/Blueprints/UI/Menu/EndGame/WBP_PXEndGameWidget.WBP_PXEndGameWidget_C"))
        (`UserWidget.AddToViewport` _returnvalue_3 0))))
  (return))

(fn `UserConstructionScript`)